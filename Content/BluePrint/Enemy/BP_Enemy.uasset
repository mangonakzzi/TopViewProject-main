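; Enemy Blueprint with a looping idle animation and a widget health bar that refills to full health whenever it is killed.
; AnyDamage subtracts health, pushes the clamped value to WBP_EnemyHPbar and sets a Dead flag at zero.
; Tick calls a custom event that turns the bar toward the player camera and, when Dead, restarts idle, restores health and clears the flag.
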(event `self.ReceiveAnyDamage`
  (params (Damage :type "Float (single-precision)") (DamageType :type "DamageType Object Reference") (InstigatedBy :type "Controller Object Reference") (DamageCauser :type "Actor Object Reference"))
  (bind _output_get (set `self.Health` (- (`self.Health`) Damage)))
  (bind _aswbp_enemy_hpbar (cast `/Game/UI/HPbar/EnemyHpbar/WBP_EnemyHPbar` (`WidgetComponent.GetWidget` (`self.Widget`))))
  (`/Game/UI/HPbar/EnemyHpbar/WBP_EnemyHPbar.HealthUI` _aswbp_enemy_hpbar (`KismetMathLibrary.FClamp` _output_get 0.0 (`self.MaxHealth`)) (`self.MaxHealth`))
  (if (<= (`self.Health`) 0.0)
    (set `self.Dead` true)))

(event `self.ReceiveBeginPlay`
  (`SkeletalMeshComponent.PlayAnimation` (`self.Mesh`) "/Game/SKnight_modular/Showcase/animations/Anim_Idle.Anim_Idle" true))

(event `self.ReceiveTick`
  (params (DeltaSeconds :type "Float (single-precision)"))
  (`self.Dead and HPbar World Location`))

(event `Dead and HPbar World Location`
  (bind _widget (`self.Widget`))
  (bind _maxhealth (`self.MaxHealth`))
  (bind _returnvalue (`KismetMathLibrary.FindLookAtRotation` (`SceneComponent.K2_GetComponentLocation` _widget) (`SceneComponent.K2_GetComponentLocation` (`PlayerCameraManager.TransformComponent` (`GameplayStatics.GetPlayerCameraManager` 0)))))
  (if (`self.Dead`)
    (`SceneComponent.K2_SetWorldRotation` _widget _returnvalue false false)
    (`SkeletalMeshComponent.PlayAnimation` (`self.Mesh`) "/Game/SKnight_modular/Showcase/animations/Anim_Idle.Anim_Idle" true)
    (bind _aswbp_enemy_hpbar (cast `/Game/UI/HPbar/EnemyHpbar/WBP_EnemyHPbar` (`WidgetComponent.GetWidget` (`self.Widget`))))
    (bind _output_get (set `self.Health` _maxhealth))
    (`/Game/UI/HPbar/EnemyHpbar/WBP_EnemyHPbar.HealthUI` _aswbp_enemy_hpbar _output_get _maxhealth)
    (set `self.Dead` false)
    (else
      (`SceneComponent.K2_SetWorldRotation` _widget _returnvalue false false))))

(fn `UserConstructionScript`)