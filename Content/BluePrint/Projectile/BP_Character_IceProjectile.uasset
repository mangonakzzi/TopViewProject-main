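; Ice projectile actor for a character that damages what it hits and then destroys itself.
; On collision, actors tagged Enemy take full damage, those tagged Team take half, and anything else takes none.
; Every hit calls the ProjectileImpact dispatcher, then spawns a water-ball impact effect and sound at the hit location.
; The construction script sets the projectile movement's initial and max speed from the Speed variable.
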(event `self.Collision.OnComponentHit`
  (params (HitComponent :type "PrimitiveComponent Object Reference") (OtherActor :type "Actor Object Reference") (OtherComp :type "PrimitiveComponent Object Reference") (NormalImpulse :type "Vector Structure") (Hit :type "HitResult Structure (by ref)"))
  (if (`self.ActorHasTag` OtherActor "Enemy")
    (`GameplayStatics.ApplyDamage` OtherActor (`self.Damage`))
    (`self.Hit Particle`)
    (elif (`self.ActorHasTag` OtherActor "Team")
      (`GameplayStatics.ApplyDamage` OtherActor (/ (`self.Damage`) 2.0))
      (`self.Hit Particle`)
      (else
        (`self.Hit Particle`)))))

(event `Hit Particle`
  (`self.ProjectileImpact` null (stale `self.Collision.OnComponentHit` Hit))
  (bind (_bblockinghit _binitialoverlap _time _distance _location) (`GameplayStatics.BreakHitResult` (stale `self.Collision.OnComponentHit` Hit)))
  (`GameplayStatics.SpawnEmitterAtLocation` "/Game/FXVarietyPack/Particles/P_ky_waterBallHit.P_ky_waterBallHit" _location)
  (`GameplayStatics.PlaySoundAtLocation` "/Engine/VREditor/Sounds/VR_ungrab_Cue.VR_ungrab_Cue" _location (struct) 1.0 1.0 0.0 null null null null)
  (`self.K2_DestroyActor`))

(fn `UserConstructionScript`
  (bind _projectilemovementcomponent (`self.ProjectileMovementComponent`))
  (set `ProjectileMovementComponent.InitialSpeed` (`self.Speed`) _projectilemovementcomponent)
  (set `ProjectileMovementComponent.MaxSpeed` (`self.Speed`) _projectilemovementcomponent))